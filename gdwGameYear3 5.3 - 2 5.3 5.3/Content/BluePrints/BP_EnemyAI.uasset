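; Enemy character that glides from its start transform to a mirror spawn point, then hunts the player and opens Level1 on contact.
; A Tick timer drives the collision-free lerp, then reveals meshes hidden from all but scene captures and switches to chasing.
; A state switch runs the intro, AIMoveTo chase with a lights-toggle call, or random-point patrol, which nothing here selects.
; Sight and sphere overlaps set flags, with sight also forcing chase after the intro.
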(event OnSeePawn(PawnSensing)
  (params (Pawn :type Pawn%20Object%20Reference))
  (Variables|Default|SetisSeeingPlayer true)
  (if (not (== (Variables|Default|GetCurStat) 0))
    (Variables|Default|SetCurStat 1)))

(event OnComponentHit(CapsuleComponent)
  (params (HitComponent :type Primitive%20Component%20Object%20Reference) (OtherActor :type Actor%20Object%20Reference) (OtherComp :type Primitive%20Component%20Object%20Reference) (NormalImpulse :type Vector :default "0, 0, 0") (Hit :type Hit%20Result%20Structure%20%28by%20ref%29))
  (Utilities|Casting|CastToBP_FirstPersonCharacter OtherActor)
  (Game|OpenLevel(byName) "Level1"))

(event OnComponentBeginOverlap(Sphere)
  (params (OverlappedComponent :type Primitive%20Component%20Object%20Reference) (OtherActor :type Actor%20Object%20Reference) (OtherComp :type Primitive%20Component%20Object%20Reference) (OtherBodyIndex :type Integer) (bFromSweep :type Boolean) (SweepResult :type Hit%20Result%20Structure%20%28by%20ref%29))
  (Utilities|Casting|CastToBP_FirstPersonCharacter OtherActor)
  (Variables|Default|SetAttack true))

(event OnComponentEndOverlap(Sphere)
  (params (OverlappedComponent :type Primitive%20Component%20Object%20Reference) (OtherActor :type Actor%20Object%20Reference) (OtherComp :type Primitive%20Component%20Object%20Reference) (OtherBodyIndex :type Integer))
  (Utilities|Casting|CastToBP_FirstPersonCharacter OtherActor)
  (Variables|Default|SetAttack false))

(event Custom|FollowPlayer
  (bind _self self)
  (AI|AIMoveTo _self "0, 0, 0" (Game|GetPlayerCharacter 0) 15.0 false
    (:then
      (Class|LightInterface|ToggleLights(Message) _self))))

(event Custom|Patrolling
  (bind _returnvalue (Transformation|GetActorLocation))
  (bind _randomlocation (AI|Navigation|GetRandomReachablePointinRadius _returnvalue 1e+03 0 0))
  (if (Variables|Default|GetHitDestination)
    (Development|PrintString (Utilities|String|ToString(Vector) _randomlocation))
    (Variables|Default|SetCurDestination _randomlocation)
    (Variables|Default|SetHitDestination false)
    (else
      (AI|AIMoveTo self (Variables|Default|GetCurDestination) 0 15.0 false
        (:OnSuccess
          (Variables|Default|SetHitDestination true))))))

(event EventBeginPlay
  (Variables|Default|SetSpawnLocationEnemy (Transformation|GetActorTransform)))

(event Collision|EventActorBeginOverlap
  (params (OtherActor :type Actor%20Object%20Reference)))

(event EventTick
  (params (DeltaSeconds :type Float%20%28single-precision%29))
  (Variables|Default|SetTimer (+ (* DeltaSeconds 0.1) (Variables|Default|GetTimer)))
  (if (> (Variables|Default|GetTimer) 0.95)
    (if (< (Variables|Default|GetTimer) 1.0)
      (Variables|Default|SetCurStat 1)
      (Class|PrimitiveComponent|SetVisibleinSceneCaptureOnly (Variables|Character|GetMesh) false)))
  (switch int (Variables|Default|GetCurStat)
    (:0
      (Transformation|SetActorTransform (Math|Transform|Lerp(Transform) (Variables|Default|GetSpawnLocationEnemy) (Variables|Default|GetMirrorSpawnLocationEnen) (Variables|Default|GetTimer)))
      (Collision|SetCollisionEnabled (Variables|Collision|GetCapsuleComponent) "NoCollision"))
    (:1
      (CallFunction|FollowPlayer)
      (Collision|SetCollisionEnabled (Variables|Collision|GetCapsuleComponent) "QueryAndPhysics" :!label _label))
    (:2
      (Development|PrintString "patrolling")
      (CallFunction|Patrolling)
      (goto _label))))

(fn ConstructionScript)