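; BP_Hammer is an interactable hammer actor that carries an outline effect built from a duplicate mesh.
; The construction script adds a static mesh component copying the object's mesh and transform, with both material slots set to Outline.
; Player overlap with the sphere adds another mesh component but assigns it no mesh, and end overlap only casts.
; Custom-depth and material-swap chains are left unconnected.
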(event OnComponentBeginOverlap(Sphere)
  (params (OverlappedComponent :type Primitive%20Component%20Object%20Reference) (OtherActor :type Actor%20Object%20Reference) (OtherComp :type Primitive%20Component%20Object%20Reference) (OtherBodyIndex :type Integer) (bFromSweep :type Boolean) (SweepResult :type Hit%20Result%20Structure%20%28by%20ref%29))
  (Utilities|Casting|CastToBP_FirstPersonCharacter OtherActor)
  (AddComponent|AddStaticMeshComponent false (Transformation|GetRelativeTransform (Variables|Default|GetObject))))

(event OnComponentEndOverlap(Sphere)
  (params (OverlappedComponent :type Primitive%20Component%20Object%20Reference) (OtherActor :type Actor%20Object%20Reference) (OtherComp :type Primitive%20Component%20Object%20Reference) (OtherBodyIndex :type Integer))
  (Utilities|Casting|CastToBP_FirstPersonCharacter OtherActor))

(event Collision|EventActorBeginOverlap
  (params (OtherActor :type Actor%20Object%20Reference))
  (|CallParentFunction OtherActor) ; This node is disabled and will not be called.\nDrag off pins to build functionality.
)

(event EventTick
  (params (DeltaSeconds :type Float%20%28single-precision%29))
  (|CallParentFunction DeltaSeconds) ; This node is disabled and will not be called.\nDrag off pins to build functionality.
)

(fn ConstructionScript
  (bind _object (Variables|Default|GetObject))
  (bind _returnvalue (AddComponent|AddStaticMeshComponent false (Transformation|GetRelativeTransform _object)))
  (bind _output_get (Variables|Default|SetNewVar _returnvalue))
  (Components|StaticMesh|SetStaticMesh _output_get (Variables|/Script/Engine.StaticMeshComponent|GetStaticMesh _object))
  (Rendering|Material|SetMaterial (Variables|Default|GetNewVar) 0 "/Game/Materials/RimLighting/Outline.Outline")
  (Rendering|Material|SetMaterial (Variables|Default|GetNewVar) 1 "/Game/Materials/RimLighting/Outline.Outline"))