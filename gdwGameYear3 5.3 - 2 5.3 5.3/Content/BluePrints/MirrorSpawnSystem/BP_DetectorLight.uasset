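; BP_DetectorLight is a point light that flickers while a BP_EnemyAI is inside its box.
; Box overlap events set EnemyInArea, and leaving the box also restores full intensity.
; Tick passes through a short Delay, then a random looping MultiGate picks one of four intensities, including off.
; FlashAlready, which this graph never sets, triggers the same flicker without an enemy present.
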(event OnComponentBeginOverlap(Box)
  (params (OverlappedComponent :type Primitive%20Component%20Object%20Reference) (OtherActor :type Actor%20Object%20Reference) (OtherComp :type Primitive%20Component%20Object%20Reference) (OtherBodyIndex :type Integer) (bFromSweep :type Boolean) (SweepResult :type Hit%20Result%20Structure%20%28by%20ref%29))
  (Utilities|Casting|CastToBP_EnemyAI OtherActor)
  (Variables|Default|SetEnemyInArea true))

(event OnComponentEndOverlap(Box)
  (params (OverlappedComponent :type Primitive%20Component%20Object%20Reference) (OtherActor :type Actor%20Object%20Reference) (OtherComp :type Primitive%20Component%20Object%20Reference) (OtherBodyIndex :type Integer))
  (Utilities|Casting|CastToBP_EnemyAI OtherActor)
  (Rendering|Components|Light|SetIntensity (Variables|Default|GetPointLight) 4e+02)
  (Variables|Default|SetEnemyInArea false))

(event EventBeginPlay)

(event Collision|EventActorBeginOverlap
  (params (OtherActor :type Actor%20Object%20Reference)))

(event EventTick
  (params (DeltaSeconds :type Float%20%28single-precision%29))
  (bind _pointlight (Variables|Default|GetPointLight))
  (Utilities|FlowControl|Delay 0.2)
  (if (Variables|Default|GetEnemyInArea)
    (Utilities|FlowControl|MultiGate true true -1 :!label _label
      (:Out%200
        (Rendering|Components|Light|SetIntensity _pointlight 4e+02))
      (:Out%201
        (Rendering|Components|Light|SetIntensity _pointlight 2e+02))
      (:Out%202
        (Rendering|Components|Light|SetIntensity _pointlight 0.0))
      (:Out%203
        (Rendering|Components|Light|SetIntensity _pointlight 1e+02)))
    (elif (Variables|Default|GetFlashAlready)
      (goto _label))))

(fn ConstructionScript)