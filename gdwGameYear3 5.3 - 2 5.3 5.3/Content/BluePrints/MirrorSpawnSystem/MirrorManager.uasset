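; MirrorManager, part of the mirror spawn system, keeps stored enemies down to one and limits how long that enemy lives.
; Tick starts a countdown for a lone enemy and destroys it after about half a minute, unless FinalMoment is set, which only prints a debug message.
; When several are stored, it destroys the first entry each tick and clears Spawned, so the remaining enemy gets a fresh countdown.
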(event EventBeginPlay)

(event EventTick
  (params (DeltaSeconds :type Float%20%28single-precision%29))
  (bind _enemystore (Variables|Default|GetEnemyStore))
  (if (== (Utilities|Array|Length (Variables|Default|GetEnemyStore)) 1)
    (if (Variables|Default|GetSpawned)
      (Variables|Default|SetEnemyCountDown (+ DeltaSeconds (Variables|Default|GetEnemyCountDown)))
      (if (>= (Variables|Default|GetEnemyCountDown) 36.0)
        (if (Variables|Default|GetFinalMoment)
          (Development|PrintString "Final Moment CHasing Forever")
          (else
            (Actor|DestroyActor (Utilities|Array|Get(acopy) _enemystore) :!label _label)
            (Utilities|Array|RemoveIndex _enemystore)
            (Variables|Default|SetSpawned false))))
      (else
        (Variables|Default|SetEnemyCountDown 0.0)
        (Variables|Default|SetSpawned true)))
    (elif (> (Utilities|Array|Length (Variables|Default|GetEnemyStore)) 1)
      (goto _label))))

(fn ConstructionScript)