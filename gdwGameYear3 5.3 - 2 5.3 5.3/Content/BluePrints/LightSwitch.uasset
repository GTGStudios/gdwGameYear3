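; Light switch actor that toggles four referenced point lights when the player interacts with it.
; Its Box overlap events enable and disable input for player controller 0, without checking which actor overlaps.
; StartInteract plays a 2D switch sound, then toggles visibility on Light3, Light4, Light2 and LightHolder.
; Each step flips the Switch boolean, but both branches make the same toggle, so the flag does not affect the lights.
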(event OnComponentBeginOverlap(Box)
  (params (OverlappedComponent :type Primitive%20Component%20Object%20Reference) (OtherActor :type Actor%20Object%20Reference) (OtherComp :type Primitive%20Component%20Object%20Reference) (OtherBodyIndex :type Integer) (bFromSweep :type Boolean) (SweepResult :type Hit%20Result%20Structure%20%28by%20ref%29))
  (Input|EnableInput (Game|GetPlayerController 0)))

(event OnComponentEndOverlap(Box)
  (params (OverlappedComponent :type Primitive%20Component%20Object%20Reference) (OtherActor :type Actor%20Object%20Reference) (OtherComp :type Primitive%20Component%20Object%20Reference) (OtherBodyIndex :type Integer))
  (Input|DisableInput (Game|GetPlayerController 0)))

(event EventBeginPlay)

(event Collision|EventActorBeginOverlap
  (params (OtherActor :type Actor%20Object%20Reference)))

(event EventTick
  (params (DeltaSeconds :type Float%20%28single-precision%29)))

(event EventStartInteract
  (bind _light_4 (Variables|Default|Getlight%204))
  (bind _lightholder (Variables|Default|GetLightHolder))
  (bind _light_2 (Variables|Default|Getlight%202))
  (bind _light_3 (Variables|Default|Getlight%203))
  (bind _pointlightcomponent (Variables|/Script/Engine.PointLight|GetPointLightComponent _light_2))
  (bind _pointlightcomponent_2 (Variables|/Script/Engine.PointLight|GetPointLightComponent _light_3))
  (bind _pointlightcomponent_3 (Variables|/Script/Engine.PointLight|GetPointLightComponent _light_4))
  (bind _pointlightcomponent_4 (Variables|/Script/Engine.PointLight|GetPointLightComponent _lightholder))
  (Audio|PlaySound2D "/Game/Sound/lightSwitch.lightSwitch" 1.0 1.0 0.0 0 0)
  (if (Variables|Default|Getswitch)
    (Rendering|ToggleVisibility _pointlightcomponent_2 false)
    (Variables|Default|Setswitch false)
    (else
      (Rendering|ToggleVisibility _pointlightcomponent_2 false)
      (Variables|Default|Setswitch true)))
  (if (Variables|Default|Getswitch)
    (Rendering|ToggleVisibility _pointlightcomponent_3 false)
    (Variables|Default|Setswitch false)
    (else
      (Rendering|ToggleVisibility _pointlightcomponent_3 false)
      (Variables|Default|Setswitch true)))
  (if (Variables|Default|Getswitch)
    (Rendering|ToggleVisibility _pointlightcomponent false)
    (Variables|Default|Setswitch false)
    (else
      (Rendering|ToggleVisibility _pointlightcomponent false)
      (Variables|Default|Setswitch true)))
  (if (Variables|Default|Getswitch)
    (Rendering|ToggleVisibility _pointlightcomponent_4 false)
    (Variables|Default|Setswitch false)
    (else
      (Rendering|ToggleVisibility _pointlightcomponent_4 false)
      (Variables|Default|Setswitch true))))

(fn ConstructionScript)