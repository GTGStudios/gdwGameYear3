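; BP_FloatActor is an interactable actor whose Sphere component moves vertically when interaction starts.
; The StartInteract event plays a timeline from the start, using its track as the lerp alpha to set the sphere's relative location between a low and a high Z position, without sweeping.
; BeginPlay, overlap and Tick are disabled placeholders, so all behavior comes from that event.
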(event EventBeginPlay
  (|CallParentFunction) ; This node is disabled and will not be called.\nDrag off pins to build functionality.
)

(event Collision|EventActorBeginOverlap
  (params (OtherActor :type Actor%20Object%20Reference))
  (|CallParentFunction OtherActor) ; This node is disabled and will not be called.\nDrag off pins to build functionality.
)

(event EventTick
  (params (DeltaSeconds :type Float%20%28single-precision%29))
  (|CallParentFunction DeltaSeconds) ; This node is disabled and will not be called.\nDrag off pins to build functionality.
)

(event EventStartInteract
  (bind _newtrack_0 (Timeline|Timeline PlayFromStart)
    (:Update
      (Transformation|SetRelativeLocation (Variables|Default|GetSphere) (Math|Vector|Lerp(Vector) "0.000000,0.000000,50.000000" (Math|Vector|MakeVector 0.0 0.0 5e+02) _newtrack_0) false false))))

(fn ConstructionScript
  (|CallParentFunction))