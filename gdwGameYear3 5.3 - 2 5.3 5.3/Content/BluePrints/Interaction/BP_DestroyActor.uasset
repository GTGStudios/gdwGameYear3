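; An interactable pickup actor that gives the player a nail and then removes itself from the world.
; On StartInteract it finds the first BP_FirstPersonCharacter via GetAllActorsOfClass, increments its TotalNails, prints the new total on screen and destroys the actor.
; BeginPlay, overlap and tick are unused.
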(event EventBeginPlay
  (|CallParentFunction) ; This node is disabled and will not be called.\nDrag off pins to build functionality.
)

(event Collision|EventActorBeginOverlap
  (params (OtherActor :type Actor%20Object%20Reference))
  (|CallParentFunction OtherActor) ; This node is disabled and will not be called.\nDrag off pins to build functionality.
)

(event EventTick
  (params (DeltaSeconds :type Float%20%28single-precision%29))
  (|CallParentFunction DeltaSeconds) ; This node is disabled and will not be called.\nDrag off pins to build functionality.
)

(event EventStartInteract
  (bind _outactors (Actor|GetAllActorsOfClass "/Game/FirstPerson/Blueprints/BP_FirstPersonCharacter.BP_FirstPersonCharacter_C"))
  (Variables|/Game/FirstPerson/Blueprints/BP_FirstPersonCharacter.BP_FirstPersonCharacter_C|SetTotalNails (Utilities|Array|Get(acopy) _outactors) (+ (Variables|/Game/FirstPerson/Blueprints/BP_FirstPersonCharacter.BP_FirstPersonCharacter_C|GetTotalNails (Utilities|Array|Get(acopy) _outactors)) 1))
  (bind _outactors_2 (Actor|GetAllActorsOfClass "/Game/FirstPerson/Blueprints/BP_FirstPersonCharacter.BP_FirstPersonCharacter_C"))
  (Development|PrintString (Utilities|String|ToString(Integer) (Variables|/Game/FirstPerson/Blueprints/BP_FirstPersonCharacter.BP_FirstPersonCharacter_C|GetTotalNails (Utilities|Array|Get(acopy) _outactors_2))))
  (Actor|DestroyActor))

(fn ConstructionScript
  (|CallParentFunction))