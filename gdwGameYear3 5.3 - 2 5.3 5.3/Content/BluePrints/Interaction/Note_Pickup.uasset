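; Collectible paper note that, on interaction, plays a paper sound and shows one of seven note screens.
; A branch chain picks the screen from the player character's PapersCollected count, so notes read in pickup order regardless of which one is found.
; It then pauses the game, shows the cursor, increments the count and destroys itself.
; The construction script duplicates the note mesh with an Outline material for highlighting.
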(event EventBeginPlay
  (|CallParentFunction) ; This node is disabled and will not be called.\nDrag off pins to build functionality.
)

(event Collision|EventActorBeginOverlap
  (params (OtherActor :type Actor%20Object%20Reference))
  (|CallParentFunction OtherActor) ; This node is disabled and will not be called.\nDrag off pins to build functionality.
)

(event EventTick
  (params (DeltaSeconds :type Float%20%28single-precision%29))
  (|CallParentFunction DeltaSeconds) ; This node is disabled and will not be called.\nDrag off pins to build functionality.
)

(event EventStartInteract
  (Audio|PlaySound2D "/Game/Sound/sound_assets/paper_sounds.paper_sounds" 1.0 1.0 0.0 0 0)
  (bind _outactors (Actor|GetAllActorsOfClass "/Game/FirstPerson/Blueprints/BP_FirstPersonCharacter.BP_FirstPersonCharacter_C"))
  (if (== (Variables|/Game/FirstPerson/Blueprints/BP_FirstPersonCharacter.BP_FirstPersonCharacter_C|GetPapersCollected (Utilities|Array|Get(acopy) _outactors)) 0)
    (bind _returnvalue (UserInterface|CreateWidget "/Game/UI/Scripts/Note_UI/1Note_Menu.1Note_Menu_C"))
    (UserInterface|Viewport|AddtoViewport _returnvalue 0 :!label _label)
    (Game|SetGamePaused true)
    (Variables|/Script/Engine.PlayerController|SetbShowMouseCursor (Game|GetPlayerController 0) true)
    (bind _outactors_2 (Actor|GetAllActorsOfClass "/Game/FirstPerson/Blueprints/BP_FirstPersonCharacter.BP_FirstPersonCharacter_C"))
    (Variables|/Game/FirstPerson/Blueprints/BP_FirstPersonCharacter.BP_FirstPersonCharacter_C|SetPapersCollected (Utilities|Array|Get(acopy) _outactors_2) (+ (Variables|/Game/FirstPerson/Blueprints/BP_FirstPersonCharacter.BP_FirstPersonCharacter_C|GetPapersCollected (Utilities|Array|Get(acopy) _outactors_2)) 1))
    (Actor|DestroyActor)
    (else
      (bind _outactors_3 (Actor|GetAllActorsOfClass "/Game/FirstPerson/Blueprints/BP_FirstPersonCharacter.BP_FirstPersonCharacter_C"))
      (if (== (Variables|/Game/FirstPerson/Blueprints/BP_FirstPersonCharacter.BP_FirstPersonCharacter_C|GetPapersCollected (Utilities|Array|Get(acopy) _outactors_3)) 1)
        (bind _returnvalue_2 (UserInterface|CreateWidget "/Game/UI/Scripts/Note_UI/2Note_Menu.2Note_Menu_C"))
        (goto _label)
        (else
          (bind _outactors_4 (Actor|GetAllActorsOfClass "/Game/FirstPerson/Blueprints/BP_FirstPersonCharacter.BP_FirstPersonCharacter_C"))
          (if (== (Variables|/Game/FirstPerson/Blueprints/BP_FirstPersonCharacter.BP_FirstPersonCharacter_C|GetPapersCollected (Utilities|Array|Get(acopy) _outactors_4)) 2)
            (bind _returnvalue_3 (UserInterface|CreateWidget "/Game/UI/Scripts/Note_UI/3Note_Menu.3Note_Menu_C"))
            (goto _label)
            (else
              (bind _outactors_5 (Actor|GetAllActorsOfClass "/Game/FirstPerson/Blueprints/BP_FirstPersonCharacter.BP_FirstPersonCharacter_C"))
              (if (== (Variables|/Game/FirstPerson/Blueprints/BP_FirstPersonCharacter.BP_FirstPersonCharacter_C|GetPapersCollected (Utilities|Array|Get(acopy) _outactors_5)) 3)
                (bind _returnvalue_4 (UserInterface|CreateWidget "/Game/UI/Scripts/Note_UI/4Note_Menu.4Note_Menu_C"))
                (goto _label)
                (else
                  (bind _outactors_6 (Actor|GetAllActorsOfClass "/Game/FirstPerson/Blueprints/BP_FirstPersonCharacter.BP_FirstPersonCharacter_C"))
                  (if (== (Variables|/Game/FirstPerson/Blueprints/BP_FirstPersonCharacter.BP_FirstPersonCharacter_C|GetPapersCollected (Utilities|Array|Get(acopy) _outactors_6)) 4)
                    (bind _returnvalue_5 (UserInterface|CreateWidget "/Game/UI/Scripts/Note_UI/5Note_Menu.5Note_Menu_C"))
                    (goto _label)
                    (else
                      (bind _outactors_7 (Actor|GetAllActorsOfClass "/Game/FirstPerson/Blueprints/BP_FirstPersonCharacter.BP_FirstPersonCharacter_C"))
                      (if (== (Variables|/Game/FirstPerson/Blueprints/BP_FirstPersonCharacter.BP_FirstPersonCharacter_C|GetPapersCollected (Utilities|Array|Get(acopy) _outactors_7)) 5)
                        (bind _returnvalue_6 (UserInterface|CreateWidget "/Game/UI/Scripts/Note_UI/6Note_Menu.6Note_Menu_C"))
                        (goto _label)
                        (else
                          (bind _outactors_8 (Actor|GetAllActorsOfClass "/Game/FirstPerson/Blueprints/BP_FirstPersonCharacter.BP_FirstPersonCharacter_C"))
                          (if (== (Variables|/Game/FirstPerson/Blueprints/BP_FirstPersonCharacter.BP_FirstPersonCharacter_C|GetPapersCollected (Utilities|Array|Get(acopy) _outactors_8)) 6)
                            (bind _returnvalue_7 (UserInterface|CreateWidget "/Game/UI/Scripts/Note_UI/7Note_Menu.7Note_Menu_C"))
                            (goto _label)))))))))))))))

(fn ConstructionScript
  (bind _note (Variables|Default|GetNote))
  (bind _returnvalue (AddComponent|AddStaticMeshComponent false (Transformation|GetRelativeTransform _note)))
  (bind _output_get (Variables|Default|SetSetStatic _returnvalue))
  (Components|StaticMesh|SetStaticMesh _output_get (Variables|/Script/Engine.StaticMeshComponent|GetStaticMesh _note))
  (Rendering|Material|SetMaterial (Variables|Default|GetSetStatic) 0 "/Game/Materials/RimLighting/Outline.Outline")
  (Rendering|Material|SetMaterial (Variables|Default|GetSetStatic) 1 "/Game/Materials/RimLighting/Outline.Outline"))