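; Wardrobe is an interactable closet that the player can step into and out of, likely as a hiding spot.
; StartInteract toggles an InsideCloset flag and teleports player character 0 to the ReferenceIn transform on entry or ReferenceOut on exit.
; Only location and rotation are applied, with no animation, input lock or other state change.
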(event EventBeginPlay)

(event Collision|EventActorBeginOverlap
  (params (OtherActor :type Actor%20Object%20Reference)))

(event EventTick
  (params (DeltaSeconds :type Float%20%28single-precision%29)))

(event EventStartInteract
  (bind _referencein (Variables|Default|GetReferenceIn))
  (bind _referenceout (Variables|Default|GetReferenceOut))
  (bind _returnvalue (Transformation|GetWorldTransform _referenceout))
  (bind _returnvalue_2 (Transformation|GetWorldTransform _referencein))
  (if (not (Variables|Default|GetInsideCloset))
    (Variables|Default|SetInsideCloset true)
    (Transformation|SetActorTransform (Game|GetPlayerCharacter 0) (Math|Transform|MakeTransform (.location _returnvalue_2) (.rotation _returnvalue_2) "1.000000,1.000000,1.000000"))
    (else
      (Variables|Default|SetInsideCloset false)
      (Transformation|SetActorTransform (Game|GetPlayerCharacter 0) (Math|Transform|MakeTransform (.location _returnvalue) (.rotation _returnvalue) "1.000000,1.000000,1.000000")))))

(fn ConstructionScript)