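; BP_Door is an interactable door that opens and closes once the player has picked up its key.
; On interact, a FlipFlop alternates playing and reversing a timeline that yaws DoorL between closed and open, with an open sound each time.
; Without the key, it plays a locked sound and shows a DoorLockedText widget for a few seconds.
; PickUpKey sets the HasKey flag.
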(event EventStartInteract
  (if (Variables|Default|GetHas%20Key?)
    (Audio|PlaySound2D "/Game/Sound/DoorOpenRadno.DoorOpenRadno" 1.0 1.0 0.0 0 0)
    (Utilities|FlowControl|FlipFlop
      (:A
        (bind _door_track (Timeline|Door%20Timeline Play)
          (:Update
            (Transformation|SetRelativeRotation (Variables|Default|GetDoorL) (Math|Rotator|MakeRotator 0.0 0.0 (Math|Float|Lerp 0.0 1e+02 _door_track)) false false))))
      (:B
        (Timeline|Door%20Timeline Reverse)))
    (else
      (Audio|PlaySound2D "/Game/Sound/DoorLocked.DoorLocked" 1.0 1.0 0.0 0 0)
      (bind _returnvalue (UserInterface|CreateWidget "/Game/3D_Assets/Door/DoorLockedText.DoorLockedText_C"))
      (UserInterface|Viewport|AddtoViewport _returnvalue 0)
      (Utilities|FlowControl|Delay 4.0)
      (Widget|RemovefromParent _returnvalue))))

(event EventPickUpKey
  (Variables|Default|SetHas%20Key? true))

(fn ConstructionScript)