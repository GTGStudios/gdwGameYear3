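; AI_Enemy is an enemy Blueprint that detects the first-person player through PawnSensing.
; When it sees BP_FirstPersonCharacter, it sets the hasSeenPlayer key on its AI controller's Blackboard to true.
; Its InCloset event calls InCloset, while BeginPlay and Interact are empty.
; Objective lookup, closet-state reset and AI MoveTo nodes are present but never run.
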(event OnSeePawn(PawnSensing)
  (params (Pawn :type Pawn%20Object%20Reference))
  (Utilities|Casting|CastToBP_FirstPersonCharacter Pawn)
  (AI|Components|Blackboard|SetValueasBool (AI|GetBlackboard (AI|GetAIController self)) (Utilities|Name|MakeLiteralName "hasSeenPlayer") true))

(event EventBeginPlay)

(event EventInCloset
  (CallFunction|InCloset))

(event EventInteract)

(fn ConstructionScript)

(fn LocateObjective
  (bind _outactors (Actor|GetAllActorsOfClass "/Game/BluePrints/BP_Objective.BP_Objective_C"))
  (Variables|Default|SetObjective (Utilities|Array|Get(acopy) _outactors)))