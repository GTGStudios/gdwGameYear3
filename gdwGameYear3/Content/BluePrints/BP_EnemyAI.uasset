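; Enemy AI character that moves from its spawn point to a mirror spawn transform, then chases the player.
; Tick lerps the transform with collision off for about four seconds, then switches state, clears the mesh's scene-capture-only visibility and enables collision.
; The chase state reissues AIMoveTo every tick.
; PawnSensing also starts the chase on sight, but its seen-player flag does not affect movement.
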(event OnSeePawn(PawnSensing)
  (params (Pawn :type Pawn%20Object%20Reference))
  (Variables|Default|SetisSeeingPlayer true)
  (CallFunction|FollowPlayer))

(event Custom|FollowPlayer
  (if (Variables|Default|GetisSeeingPlayer)
    _
    (else
      _))
  (AI|AIMoveTo self "0, 0, 0" (Game|GetPlayerCharacter 0) 15.0 false))

(event EventBeginPlay
  (Variables|Default|SetSpawnLocationEnemy (Transformation|GetActorTransform)))

(event Collision|EventActorBeginOverlap
  (params (OtherActor :type Actor%20Object%20Reference)))

(event EventTick
  (params (DeltaSeconds :type Float%20%28single-precision%29))
  (Variables|Default|SetTimer (+ (* DeltaSeconds 0.2) (Variables|Default|GetTimer)))
  (if (> (Variables|Default|GetTimer) 0.8)
    (if (< (Variables|Default|GetTimer) 0.9)
      (Variables|Default|SetCurStat 1)
      (Class|PrimitiveComponent|SetVisibleinSceneCaptureOnly (Variables|Character|GetMesh) false)))
  (switch int (Variables|Default|GetCurStat)
    (:0
      (Transformation|SetActorTransform (Math|Transform|Lerp(Transform) (Variables|Default|GetSpawnLocationEnemy) (Variables|Default|GetMirrorSpawnLocationEnen) (Variables|Default|GetTimer)))
      (Collision|SetCollisionEnabled (Variables|Collision|GetCapsuleComponent) "NoCollision"))
    (:1
      (CallFunction|FollowPlayer)
      (Collision|SetCollisionEnabled (Variables|Collision|GetCapsuleComponent) "QueryAndPhysics"))))

(fn ConstructionScript)