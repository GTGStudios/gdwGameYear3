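; Sample enemy for a mirror spawn system that slides from its spawn transform to a mirror spawn transform while chasing the player.
; Tick advances a scaled timer as the lerp alpha, then near the end switches state and clears the mannequin's scene-capture-only visibility.
; BeginPlay issues AIMoveTo on the player immediately, alongside the lerp.
; LocateObjective and FollowPlayer are empty, and the spawn-transform capture is unwired.
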(event EventBeginPlay
  (CallFunction|LocateObjective)
  (AI|AIMoveTo self "0, 0, 0" (Game|GetPlayerCharacter 0) 2.0 false))

(event Collision|EventActorBeginOverlap
  (params (OtherActor :type Actor%20Object%20Reference)))

(event EventTick
  (params (DeltaSeconds :type Float%20%28single-precision%29))
  (Variables|Default|SetTimer (+ (* DeltaSeconds 0.2) (Variables|Default|GetTimer)))
  (if (> (Variables|Default|GetTimer) 0.8)
    (if (< (Variables|Default|GetTimer) 0.9)
      (Variables|Default|SetCurStat 1)
      (Class|PrimitiveComponent|SetVisibleinSceneCaptureOnly (Variables|Default|GetSK_Mannequin) false)))
  (switch int (Variables|Default|GetCurStat)
    (:0
      (Transformation|SetActorTransform (Math|Transform|Lerp(Transform) (Variables|Default|GetSpawnLocationEnemy) (Variables|Default|GetMirrorSpawnLocationEnemy) (Variables|Default|GetTimer)))
      (Development|PrintString "lerping"))))

(fn ConstructionScript)

(fn FollowPlayer)

(fn LocateObjective)